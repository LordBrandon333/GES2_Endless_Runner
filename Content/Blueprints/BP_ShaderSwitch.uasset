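; BP_ShaderSwitch is a hit-triggered switch that changes which post-process volume applies globally.
; On BeginPlay it gathers every PostProcessVolume and leaves only the first one unbound.
; A hit on its Box moves the unbound flag to the next volume, wrapping at the end, with debug prints of count and index.
; A DoOnce with no reset limits each instance to a single switch.
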(event `self.ReceiveBeginPlay`
  (bind _outactors (`GameplayStatics.GetAllActorsOfClass` "/Script/Engine.PostProcessVolume"))
  (bind _output_get (set `self.AllVolumes` _outactors))
  (`KismetSystemLibrary.PrintString` (`KismetStringLibrary.Conv_IntToString` (`KismetArrayLibrary.Array_Length` _output_get)))
  (for _array_element _output_get
    (set `PostProcessVolume.bUnbound` false _array_element))
  (set `PostProcessVolume.bUnbound` true (`|GetArrayItem` _output_get))
  (set `self.CurrentActiveIndex` 0))

(event `self.Box.OnComponentHit`
  (params (HitComponent :type "PrimitiveComponent Object Reference") (OtherActor :type "Actor Object Reference") (OtherComp :type "PrimitiveComponent Object Reference") (NormalImpulse :type "Vector Structure") (Hit :type "HitResult Structure (by ref)"))
  (bind _allvolumes (`self.AllVolumes`))
  (bind _currentactiveindex (`self.CurrentActiveIndex`))
  (`/Engine/EditorBlueprintResources/StandardMacros.DoOnce` false
    (:`Completed`
      (set `PostProcessVolume.bUnbound` false (`|GetArrayItem` _allvolumes _currentactiveindex))
      (`/Engine/EditorBlueprintResources/StandardMacros.IncrementInt` _currentactiveindex
        (:`  `
          (`KismetSystemLibrary.PrintString` (`KismetStringLibrary.Conv_IntToString` (`self.CurrentActiveIndex`)))
          (if (not (< _currentactiveindex (`KismetArrayLibrary.Array_Length` _allvolumes)))
            (set `self.CurrentActiveIndex` 0))
          (set `PostProcessVolume.bUnbound` true (`|GetArrayItem` (`self.AllVolumes`) (`self.CurrentActiveIndex`))))))))

(fn `UserConstructionScript`)