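; Player character for an endless runner: Granny moves along the camera's forward vector, gradually speeds up, and can jump or slide.
; Jump and slide functions resize the capsule and offset the spring arm or mesh, with paired end functions to restore them.
; Begin play stores the start position and shows the score widget.
; Hitting an obstacle flags a head or foot hit, stops movement input, then opens the death screen after a delay.
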(event `self.ReceiveBeginPlay`
  (set `self.StartingPos` (`SceneComponent.K2_GetComponentLocation` (`self.CapsuleComponent`)))
  (bind _returnvalue (`|CreateWidget` "/Game/UI/UW_Score.UW_Score_C"))
  (`UserWidget.AddToViewport` _returnvalue 0))

(event `self.CapsuleComponent.OnComponentHit`
  (params (HitComponent :type "PrimitiveComponent Object Reference") (OtherActor :type "Actor Object Reference") (OtherComp :type "PrimitiveComponent Object Reference") (NormalImpulse :type "Vector Structure") (Hit :type "HitResult Structure (by ref)"))
  (bind (_bblockinghit _binitialoverlap _time _distance _location _impactpoint _normal _impactnormal _physmat _hitactor) (`GameplayStatics.BreakHitResult` Hit))
  (castclass `/Game/Blueprints/BP_Obstacle` (`GameplayStatics.GetObjectClass` _hitactor))
  (if (> (.z _impactpoint) (`CapsuleComponent.CapsuleHalfHeight` (`self.CapsuleComponent`)))
    (set `self.HitHead` true)
    (else
      (set `self.HitFoot` true)))
  (set `self.Hit` true)
  (`KismetSystemLibrary.Delay` 4.0)
  (`GameplayStatics.OpenLevel` "DeathScreenMap"))

(fn `InfiniteRun`
  (if (not (`self.Hit`))
    (`self.AddMovementInput` (`SceneComponent.GetForwardVector` (`self.Camera`)))
    ; Increase speed over time
    (bind _result (`/Engine/EditorBlueprintResources/StandardMacros.IncrementFloat` (`self.TickCounter`))
      (:`  `
        (if (> _result 5.0)
          (`/Engine/EditorBlueprintResources/StandardMacros.IncrementFloat` (`CharacterMovementComponent.MaxWalkSpeed` (`self.CharacterMovement`))
            (:`  `
              (set `self.TickCounter` 0.0))))))))

(fn `Jumping`
  (bind _springarm (`self.SpringArm`))
  (if (and (not (`self.IsSliding`)) (> (`KismetSystemLibrary.GetGameTimeInSeconds`) (+ (`self.LastJumpTime`) 1.0)))
    (`SceneComponent.K2_SetWorldLocation` _springarm (- (`SceneComponent.K2_GetComponentLocation` _springarm) (`KismetMathLibrary.MakeVector` 0.0 0.0 (/ (`self.BaseHalfHeight`) 2.0))) false false)
    (`self.Jump`)
    (`CapsuleComponent.SetCapsuleHalfHeight` (`self.CapsuleComponent`) 44.0 true)
    (set `self.LastJumpTime` (`KismetSystemLibrary.GetGameTimeInSeconds`))))

(fn `OnHitHead`
  (`CapsuleComponent.SetCapsuleHalfHeight` (`self.CapsuleComponent`) 88.0 true))

(fn `OnJumpEnd`
  (bind _springarm (`self.SpringArm`))
  (`CapsuleComponent.SetCapsuleHalfHeight` (`self.CapsuleComponent`) 88.0 true)
  (`SceneComponent.K2_SetWorldLocation` _springarm (+ (`SceneComponent.K2_GetComponentLocation` _springarm) (`KismetMathLibrary.MakeVector` 0.0 0.0 (/ (`self.BaseHalfHeight`) 2.0))) false false))

(fn `OnSlideEnd`
  (bind _capsulecomponent (`self.CapsuleComponent`))
  (bind _mesh (`self.Mesh`))
  ; Enable input and reset collider location / height
  (`self.EnableInput` null)
  (`SceneComponent.K2_SetWorldLocation` _capsulecomponent (+ (`SceneComponent.K2_GetComponentLocation` _capsulecomponent) (`KismetMathLibrary.MakeVector` 0.0 0.0 (/ (`self.BaseHalfHeight`) 2.0))) false false)
  (`CapsuleComponent.SetCapsuleHalfHeight` _capsulecomponent (`self.BaseHalfHeight`) true)
  ; Reset Mesh height and deactivate bool
  (`SceneComponent.K2_SetWorldLocation` _mesh (- (`SceneComponent.K2_GetComponentLocation` _mesh) (`KismetMathLibrary.MakeVector` 0.0 0.0 (`self.ZChange`))) false false)
  (set `self.IsSliding` false))

(fn `Sliding`
  (bind _capsulecomponent (`self.CapsuleComponent`))
  (bind _mesh (`self.Mesh`))
  (if (and (not (`self.IsSliding`)) (not (`NavMovementInterface.IsFalling` (`self.CharacterMovement`))))
    ; Set new half height and location of collider, so its smaller and on the ground
    (`self.DisableInput` null)
    (`CapsuleComponent.SetCapsuleHalfHeight` _capsulecomponent (/ (`self.BaseHalfHeight`) 4.0) true)
    (`SceneComponent.K2_SetWorldLocation` _capsulecomponent (- (`SceneComponent.K2_GetComponentLocation` _capsulecomponent) (0.0 0.0 33.0)) false false)
    ; Move mesh to new correct height
    (`SceneComponent.K2_SetWorldLocation` _mesh (+ (`SceneComponent.K2_GetComponentLocation` _mesh) (`KismetMathLibrary.MakeVector` 0.0 0.0 (`self.ZChange`))) false false)
    (set `self.IsSliding` true)))

(fn `TeleportToStartPosition`
  (`SceneComponent.K2_SetWorldLocation` (`self.CapsuleComponent`) (`self.StartingPos`) false false))

(fn `UserConstructionScript`)