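; Player controller for an endless runner that drives the BP_Character_Granny actor.
; On BeginPlay it adds the IMC_Controls Enhanced Input mapping context and caches the Granny found with GetActorOfClass, rather than using the possessed pawn.
; It calls InfiniteRun on her every Tick and forwards the jump and slide input actions to her Jumping and Sliding functions.
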(event `self.ReceiveBeginPlay`
  (`EnhancedInputSubsystemInterface.AddMappingContext` (subsystem `EnhancedInputLocalPlayerSubsystem`) "/Game/Blueprints/IMC_Controls.IMC_Controls" 0 (struct))
  (bind _returnvalue (`GameplayStatics.GetActorOfClass` "/Game/Blueprints/BP_Character_Granny.BP_Character_Granny_C"))
  (set `self.OwningActor` _returnvalue))

(event `self.ReceiveTick`
  (params (DeltaSeconds :type "Float (single-precision)"))
  (`/Game/Blueprints/BP_Character_Granny.InfiniteRun` (`self.OwningActor`)))

(event `EnhancedInput|/Game/Blueprints/IA_Jump`
  (params (ActionValue :type Boolean) (ElapsedSeconds :type "Float (double-precision)") (TriggeredSeconds :type "Float (double-precision)") (InputAction :type "InputAction Object Reference" :default "/Game/Blueprints/IA_Jump.IA_Jump"))
  (:`Triggered`
    (`/Game/Blueprints/BP_Character_Granny.Jumping` (`self.OwningActor`))))

(event `EnhancedInput|/Game/Blueprints/IA_Slide`
  (params (ActionValue :type Boolean) (ElapsedSeconds :type "Float (double-precision)") (TriggeredSeconds :type "Float (double-precision)") (InputAction :type "InputAction Object Reference" :default "/Game/Blueprints/IA_Slide.IA_Slide"))
  (:`Triggered`
    (`/Game/Blueprints/BP_Character_Granny.Sliding` (`self.OwningActor`))))

(fn `UserConstructionScript`)